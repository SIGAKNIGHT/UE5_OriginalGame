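; Temporary boss enemy that shows a boss HP bar on screen with a placeholder name.
; BeginPlay creates the BossHP_WBP widget, adds it to the viewport and sends it the enemy name.
; Tick polls BPHP, pushes current and last HP to the widget as fractions of max HP, and debug-prints the boss HP through StatusPrintString.
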(event `self.ReceiveBeginPlay`
  (`|ExecutionSequence`
    (:`then_0`
      ;[1 1 1] HPゲージ作成
      (bind _returnvalue (`|CreateWidget` "/Game/MaedaDaiki/Blueprints/BossHP_WBP.BossHP_WBP_C"))
      (bind _output_get (set `self.BossHP_Widget` _returnvalue))
      (`Widget.SetVisibility` _output_get "Visible")
      (`UserWidget.AddToViewport` _output_get 0))
    (:`then_1`
      ;[1 1 1] 名前設定
      (bind _output_get_2 (set `self.EnemyName` "ぼすーーーーー"))
      (`/Game/MaedaDaiki/Blueprints/BossHP_WBP.DispSetEnemyName_Event` (`self.BossHP_Widget`) _output_get_2))))

(event `self.ReceiveTick`
  (params (DeltaSeconds :type "Float (single-precision)"))
  (bind _bp_hp (`self.BP_HP`))
  (bind _bp_hp_2 (`self.BP_HP`))
  (bind _bp_hp_3 (`self.BP_HP`))
  (`|ExecutionSequence`
    (:`then_1`
      ;[1 1 1] コメント
      (set `/Game/MaedaDaiki/Blueprints/BossHP_WBP.WBP_HP` (/ (`/Game/Blueprints/Player/BP_HP.HP` _bp_hp) (`/Game/Blueprints/Player/BP_HP.MaxHP` _bp_hp)) (`self.BossHP_Widget`))
      (set `/Game/MaedaDaiki/Blueprints/BossHP_WBP.WBP_LastHP` (/ (`/Game/Blueprints/Player/BP_HP.LastHP` _bp_hp_2) (`/Game/Blueprints/Player/BP_HP.MaxHP` _bp_hp_2)) (`self.BossHP_Widget`))
      (`KismetSystemLibrary.PrintString` (`self.StatusPrintString` "BossHP" (`/Game/Blueprints/Player/BP_HP.HP` _bp_hp_3) (`/Game/Blueprints/Player/BP_HP.MaxHP` _bp_hp_3)) true false (struct :`R` 0.6 :`A` 1.0) 0.0))))

(fn `UserConstructionScript`)