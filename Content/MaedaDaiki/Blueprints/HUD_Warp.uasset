(event `self.ReceiveBeginPlay`
  (bind _returnvalue (`GameplayStatics.GetPlayerController` 0))
  ;[1 1 1] 非表示でUI生成
  (`|ExecutionSequence`
    (:`then_0`
      (bind _returnvalue_2 (`|CreateWidget` "/Game/MaedaDaiki/Blueprints/WBP_Warp.WBP_Warp_C" _returnvalue))
      (bind _output_get (set `self.WarpMenuWidget` _returnvalue_2))
      (`Widget.SetVisibility` _returnvalue_2 "Collapsed")
      (`UserWidget.AddToViewport` _returnvalue_2 0)
      (`UserWidget.AddToViewport` _output_get 0))
    (:`then_1`
      (bind _returnvalue_3 (`|CreateWidget` "/Game/MaedaDaiki/Blueprints/WBP_Warpicon.WBP_Warpicon_C" _returnvalue))
      (bind _output_get_2 (set `self.WarpiconWidget` _returnvalue_3))
      (`Widget.SetVisibility` _output_get_2 "Collapsed")
      (`UserWidget.AddToViewport` _output_get_2 0))
    (:`then_2`
      (bind _returnvalue_4 (`|CreateWidget` "/Game/MaedaDaiki/Blueprints/WBP_BossWall.WBP_BossWall_C" _returnvalue))
      (bind _output_get_3 (set `self.BossWallWidget` _returnvalue_4))
      (`Widget.SetVisibility` _output_get_3 "Collapsed")
      (`UserWidget.AddToViewport` _output_get_3 900))
    (:`then_3`
      (bind _returnvalue_5 (`|CreateWidget` "/Game/MaedaDaiki/Blueprints/WBP_Fade.WBP_Fade_C" _returnvalue))
      (bind _output_get_4 (set `self.FadeWidget` _returnvalue_5))
      (`Widget.SetVisibility` _output_get_4 "Visible")
      (`UserWidget.AddToViewport` _output_get_4 0)
      (`UserWidget.PlayAnimation` _output_get_4 (`/Game/MaedaDaiki/Blueprints/WBP_Fade.fade` _output_get_4) 0.0 1 "Reverse" 0.5 false)
      (`KismetSystemLibrary.Delay` 3.0)
      (`Widget.SetVisibility` _output_get_4 "Hidden"))
    (:`then_4`
      (bind _returnvalue_6 (`|CreateWidget` "/Game/UI/WBP_YOUDIED.WBP_YOUDIED_C" _returnvalue))
      (bind _output_get_5 (set `self.YouDiedWidget` _returnvalue_6))
      (`Widget.SetVisibility` _output_get_5 "Collapsed")
      (`UserWidget.AddToViewport` _output_get_5 0))
    (:`then_5`
      (bind _returnvalue_7 (`|CreateWidget` "/Game/UI/WBP_HUNTED.WBP_HUNTED_C" _returnvalue))
      (bind _output_get_6 (set `self.YouHuntedWidget` _returnvalue_7))
      (`Widget.SetVisibility` _output_get_6 "Collapsed")
      (`UserWidget.AddToViewport` _output_get_6 0))))

(event `DispYouDied_Event`
  (bind _youdiedwidget (`self.YouDiedWidget`))
  ;[1 1 1] YOU_DIED表示アニメーション
  (`Widget.SetVisibility` _youdiedwidget "Visible")
  (`UserWidget.PlayAnimation` _youdiedwidget (`/Game/UI/WBP_YOUDIED.YOU_DIED` _youdiedwidget) 0.0 1 "Forward" 0.5 false))

(event `DispYouHunted_Event`
  (bind _youhuntedwidget (`self.YouHuntedWidget`))
  ;[1 1 1] YOU_HUNTED表示アニメーション
  (`Widget.SetVisibility` _youhuntedwidget "Visible")
  (`UserWidget.PlayAnimation` _youhuntedwidget (`/Game/UI/WBP_HUNTED.YOU_HUNTED` _youhuntedwidget) 0.0 1 "Forward" 0.5 false))

(event `DispWarpMenu_Event`
  (params (IsWarpMenu :type Boolean))
  ;[1 1 1] ワープメニューを表示
  (if IsWarpMenu
    (`|ExecutionSequence`
      (:`then_0`
        (bind _warpmenuwidget (`self.WarpMenuWidget`)
          (:`then`
            (`Widget.SetVisibility` _warpmenuwidget "Visible")
            (`WidgetBlueprintLibrary.SetInputMode_GameAndUIEx` (`self.GetOwningPlayerController`) _warpmenuwidget "DoNotLock" true true)
            (set `self.IsShowWarpMenu` true))
          (:`else`)))
      (:`then_1`
        (`GameplayStatics.SetGamePaused` true) ; ポーズ状態にする
      ))
    (else
      ;[1 1 1] ワープメニューを非表示に
      (`GameplayStatics.SetGamePaused` false)
      (`WidgetBlueprintLibrary.SetInputMode_GameOnly` (`self.GetOwningPlayerController`))
      (bind _warpmenuwidget_2 (`self.WarpMenuWidget`)
        (:`then`
          (`Widget.SetVisibility` _warpmenuwidget_2 "Collapsed")
          (set `self.IsShowWarpMenu` false)
          (set `self.WarpMenuHiddenTimer` 0.1))
        (:`else`)))))

(event `DispWarpicon_Event`
  (params (IsWarpicon :type Boolean))
  ;[1 1 1] ワープアイコン
  ;;[1 1 1] ワープメニュー表示中は非表示に
  (if (`self.IsShowWarpMenu`)
    ;;[1 1 1] 非表示
    (bind _warpiconwidget (`self.WarpiconWidget` :!label _label)
      (:`then`
        (`Widget.SetVisibility` _warpiconwidget "Collapsed"))
      (:`else`))
    (elif IsWarpicon
      ;;[1 1 1] Warpicon表示
      (bind _warpiconwidget_2 (`self.WarpiconWidget`)
        (:`then`
          (`Widget.SetVisibility` _warpiconwidget_2 "Visible"))
        (:`else`))
      (else
        (goto _label)))))

(event `DispBossWall_Event`
  (params (IsBossWall :type Boolean) (delataTime :type "Float (double-precision)"))
  (bind _bosswallalpha (`self.BossWallAlpha`))
  ;[1 1 1] ボス壁のUI
  (if IsBossWall
    ;;[1 1 1] 表示
    (bind _bosswallwidget (`self.BossWallWidget`)
      (:`then`
        (`Widget.SetVisibility` _bosswallwidget "Visible")
        (bind _output_get (set `self.BossWallAlpha` (`KismetMathLibrary.FMin` (+ (`self.BossWallAlpha`) (* delataTime 5.0)) 1.0)))
        (`Image.SetBrushTintColor` (`/Game/MaedaDaiki/Blueprints/WBP_BossWall.Image_225` (`self.BossWallWidget`)) (make `SlateColor` (make `LinearColor` 1.0 1.0 1.0 _output_get))))
      (:`else`))
    (else
      ;;[1 1 1] 非表示
      (if (<= _bosswallalpha 0.0)
        (bind _bosswallwidget_2 (`self.BossWallWidget`)
          (:`then`
            (`Widget.SetVisibility` _bosswallwidget_2 "Collapsed"))
          (:`else`))
        (else
          (bind _output_get_2 (set `self.BossWallAlpha` (`KismetMathLibrary.FMax` (- _bosswallalpha (* delataTime 5.0)))))
          (`Image.SetBrushTintColor` (`/Game/MaedaDaiki/Blueprints/WBP_BossWall.Image_225` (`self.BossWallWidget`)) (make `SlateColor` (make `LinearColor` 1.0 1.0 1.0 _output_get_2))))))))

(event `self.ReceiveTick`
  (params (DeltaSeconds :type "Float (single-precision)"))
  (bind _output_get (set `self.WarpMenuHiddenTimer` (- (`self.WarpMenuHiddenTimer`) DeltaSeconds)))
  (if (<= _output_get 0.0)
    (set `self.WarpMenuHiddenTimer` 0.0)))

(fn `UserConstructionScript`)