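; Child enemy Blueprint for the "Taurus Demon" that plays a scripted intro once active and has its own attack and death.
; Tick prints and switches on an enum state: wait, walk forward for a second, roar, then idle, which has no handler here.
; DoOnce-gated montages drive the roar and a swipe attack, which this graph never calls.
; Death calls the parent with a montage, then spawns Niagara particles and timeline-fades the material before hiding the mesh.
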(event `self.Active`
  (`parent.Active`))

(event `self.ReceiveBeginPlay`
  (set `self.EnemyName` "Taurus Demon")
  (`parent.ReceiveBeginPlay`))

(event `self.ReceiveTick`
  (params (DeltaSeconds :type "Float (single-precision)"))
  (bind _enemyenum_0 (`self.EnemyEnum_0`))
  ;[1 1 1] Tick
  (`parent.ReceiveTick` DeltaSeconds)
  (`KismetSystemLibrary.PrintString` (`|GetEnumeratorNameAsString` _enemyenum_0))
  (switch `/Game/Blueprints/Enemy/EnemyEnum` _enemyenum_0
    (:`NewEnumerator0`
      (`self.Wait`))
    (:`NewEnumerator1`
      (`self.WalkForward`))
    (:`NewEnumerator2`
      (`self.Roar`))))

(event `self.Wait`
  (if (`self.IsActive`)
    (set `self.EnemyEnum_0` "NewEnumerator1")))

(event `self.AttackR1`
  (`/Engine/EditorBlueprintResources/StandardMacros.DoOnce` false :!label _label
    (:`Completed`
      (`|PlayMontage` (`self.Mesh`) "/Game/AnimMontage/MawJLaygo/mutantswiping_UE_Montage.mutantswiping_UE_Montage"
        (:`OnCompleted`
          (goto _label :!via `Reset`))))))

(event `self.Death`
  (params (MontageToPlay :type "AnimMontage Object Reference"))
  (bind _mesh (`self.Mesh`))
  (bind _mesh_2 (`self.Mesh`))
  (`parent.Death` "/Game/AnimMontage/MawJLaygo/StandingReactDeathForward_UE_Montage.StandingReactDeathForward_UE_Montage")
  (`KismetSystemLibrary.Delay` 3.0)
  (`|ExecutionSequence`
    (:`then_0`
      (`NiagaraFunctionLibrary.SpawnSystemAttached` "/Game/MaedaDaiki/Blueprints/DeathNiagaraSystem.DeathNiagaraSystem" (`self.Mesh`) "None" (0.0 0.0 0.0) (struct) "SnapToTarget" true :!pinned true) ; パーティクル生成
    )
    (:`then_1`
      (`PrimitiveComponent.SetMaterial` _mesh_2 0 "/Game/MaedaDaiki/Material/MAW_MAT_Death.MAW_MAT_Death" :!pinned true) ; マテリアルを徐々に半透明にする
      (`PrimitiveComponent.CreateDynamicMaterialInstance` _mesh_2 0 null "None")
      (bind (_direction _fade) (`Timeline|FadeTime`)
        (:`Update`
          (`MeshComponent.SetScalarParameterValueOnMaterials` _mesh "Opacity" _fade))
        (:`Finished`
          (`SceneComponent.SetVisibility` _mesh false false))))))

(event `WalkForward`
  (`self.Move` 0.5)
  (`KismetSystemLibrary.Delay` 1.0)
  (set `self.EnemyEnum_0` "NewEnumerator2"))

(event `Roar`
  (if (not (`self.IsFalling`))
    (`/Engine/EditorBlueprintResources/StandardMacros.DoOnce` false :!label _label_2
      (:`Completed`
        (`|PlayMontage` (`self.Mesh`) "/Game/AnimMontage/MawJLaygo/mutantroaring_UE_Montage.mutantroaring_UE_Montage" 1.5
          (:`OnCompleted`
            (set `self.EnemyEnum_0` "NewEnumerator3")
            (goto _label_2 :!via `Reset`)))))))

(fn `UserConstructionScript`
  (`parent.UserConstructionScript`))