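; WarpUI handles the player-facing prompt and menu for warp points, using overlaps between Sphere2 and Warp_Point actors.
; Every Tick it polls the overlap and tells HUD_Warp to show or hide the warp icon, using IsWarpicon as a per-frame flag.
; The IA_E input repeats the overlap check while the game is unpaused and opens the warp menu through the same HUD.
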(event `EnhancedInput|/Game/Input/IA_E`
  (params (ActionValue :type Boolean) (ElapsedSeconds :type "Float (double-precision)") (TriggeredSeconds :type "Float (double-precision)") (InputAction :type "InputAction Object Reference" :default "/Game/Input/IA_E.IA_E"))
  ;[1 1 1] Qキーを押したときにプレイヤーの前方にワープオブジェクトがあったらワープメニューを表示
  (:`Triggered`
    ;;[1 1 1] ループで当たっているかを調べる
    (if (not (`GameplayStatics.IsGamePaused`))
      (for _ (`PrimitiveComponent.GetOverlappingActors` (`self.Sphere2`) "/Game/MaedaDaiki/Blueprints/Warp_Point.Warp_Point_C")
        (bind _ashud_warp (cast `/Game/MaedaDaiki/Blueprints/HUD_Warp` (`PlayerController.GetHUD` (`GameplayStatics.GetPlayerController` 0))))
        (`/Game/MaedaDaiki/Blueprints/HUD_Warp.DispWarpMenu_Event` _ashud_warp true)
        (break)))))

(event `self.ReceiveTick`
  (params (DeltaSeconds :type "Float (single-precision)"))
  ;[1 1 1] ワープIcon表示非表示
  (for _ (`PrimitiveComponent.GetOverlappingActors` (`self.Sphere2`) "/Game/MaedaDaiki/Blueprints/Warp_Point.Warp_Point_C")
    (bind _ashud_warp (cast `/Game/MaedaDaiki/Blueprints/HUD_Warp` (`PlayerController.GetHUD` (`GameplayStatics.GetPlayerController` 0))))
    (`/Game/MaedaDaiki/Blueprints/HUD_Warp.DispWarpicon_Event` _ashud_warp true) ; Icon表示
    (set `self.IsWarpicon` true)
    (break))
  (if (`self.IsWarpicon`)
    (set `self.IsWarpicon` false)
    (else
      (bind _ashud_warp_2 (cast `/Game/MaedaDaiki/Blueprints/HUD_Warp` (`PlayerController.GetHUD` (`GameplayStatics.GetPlayerController` 0))))
      (`/Game/MaedaDaiki/Blueprints/HUD_Warp.DispWarpicon_Event` _ashud_warp_2 false) ; Icon非表示
    )))