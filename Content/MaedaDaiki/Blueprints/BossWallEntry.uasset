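; BossWallEntry handles the player passing through a boss fog wall into the boss room.
; Each Tick outside the room, sphere overlap with Boss_Wall toggles the HUD_Warp prompt and caches the wall's EnterPosition.
; Pressing E while prompted snaps TargetActor there, keeping its height, then nudges it forward per frame without collision.
; When the timer expires, collision returns and IsInBossStage is set; debug prints trace the flags.
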(event `Key|E`
  (params (Key :type "Key Structure"))
  (:`Pressed`
    ;[1 1 1] ボス部屋外なら
    (if (not (`self.IsInBossStage`))
      ;[1 1 1] UIが出ている状態で
      (if (`self.IsBossWallEntry`)
        (set `self.IsBossWallDecision` true)))))

(event `self.ReceiveTick`
  (params (DeltaSeconds :type "Float (single-precision)"))
  (bind (_bosswallposition_x _bosswallposition_y) (`KismetMathLibrary.BreakVector` (`self.BossWallPosition`)))
  (bind _targetactor (`self.TargetActor`))
  (bind _bosswall_timer (`self.BossWall Timer`))
  (bind (_returnvalue_x _returnvalue_y _returnvalue_z) (`KismetMathLibrary.BreakVector` (`Actor.K2_GetActorLocation` (`self.TargetActor`))))
  (`|ExecutionSequence`
    (:`then_0`
      (`KismetSystemLibrary.PrintString` (`KismetStringLibrary.BuildString_Bool` "IsBossWallDecision:" "" (`self.IsBossWallDecision`)) true true (struct :`R` 1.0 :`A` 1.0) 0.0)
      (`KismetSystemLibrary.PrintString` (`KismetStringLibrary.BuildString_Bool` "IsBossWallEntry:" "" (`self.IsBossWallEntry`)) true true (struct :`R` 1.0 :`A` 1.0) 0.0)
      (`KismetSystemLibrary.PrintString` (`KismetStringLibrary.BuildString_Bool` "IsInBossStage:" "" (`self.IsInBossStage`)) true true (struct :`R` 1.0 :`A` 1.0) 0.0))
    (:`then_1`
      ;[1 1 1] ボス部屋内じゃないなら
      (if (not (`self.IsInBossStage`))
        (`|ExecutionSequence`
          (:`then_0`
            ;[1 1 1] 霧抜け
            (if (`self.IsBossWallDecision`)
              (`KismetSystemLibrary.PrintString` (`KismetStringLibrary.Conv_DoubleToString` _bosswall_timer) true true (struct :`G` 1.0 :`A` 1.0) 0.0)
              (set `self.BossWall Timer` (- _bosswall_timer DeltaSeconds))
              (if (> (`self.BossWall Timer`) 0.0)
                ;;[1 1 1] プレイヤーを壁の任意の位置にもっと来るー＞前に移動させる
                (switch `int` (`self.BossWallMoveState`)
                  (:`0`
                    (bind _output_get (set `self.BossWallPosition` (`KismetMathLibrary.MakeVector` _bosswallposition_x _bosswallposition_y _returnvalue_z)))
                    (`Actor.K2_SetActorLocationAndRotation` :`self` (`self.TargetActor`) :`NewLocation` _output_get)
                    (set `self.BossWallMoveState` 1))
                  (:`1`
                    (`Actor.SetActorEnableCollision` _targetactor false)
                    (`Actor.K2_AddActorLocalOffset` _targetactor (2.0 0.0 0.0) false false)))
                (else
                  (set `self.IsBossWallDecision` false)
                  (set `self.BossWall Timer` 2.0)
                  (`Actor.SetActorEnableCollision` _targetactor true)
                  (set `self.BossWallMoveState` 0)
                  (set `self.IsInBossStage` true) ; ボス部屋に入った
                ))))
          (:`then_1`
            ;[1 1 1] BossWallアイコン表示、非表示
            (for _array_element (`PrimitiveComponent.GetOverlappingActors` (`self.Sphere`) "/Game/MaedaDaiki/Blueprints/Boss_Wall.Boss_Wall_C")
              (bind _ashud_warp (cast `/Game/MaedaDaiki/Blueprints/HUD_Warp` (`PlayerController.GetHUD` (`GameplayStatics.GetPlayerController` 0))))
              (`/Game/MaedaDaiki/Blueprints/HUD_Warp.DispBossWall_Event` _ashud_warp true)
              (set `self.IsBossWallEntry` true)
              (bind _asboss_wall (cast `/Game/MaedaDaiki/Blueprints/Boss_Wall` _array_element))
              (set `self.BossWallPosition` (`SceneComponent.K2_GetComponentLocation` (`/Game/MaedaDaiki/Blueprints/Boss_Wall.EnterPosition` _asboss_wall)))
              (set `self.IsWallIcon` true)
              (break))
            (if (`self.IsWallIcon`)
              (set `self.IsWallIcon` false)
              (else
                (bind _ashud_warp_2 (cast `/Game/MaedaDaiki/Blueprints/HUD_Warp` (`PlayerController.GetHUD` (`GameplayStatics.GetPlayerController` 0))))
                (`/Game/MaedaDaiki/Blueprints/HUD_Warp.DispBossWall_Event` _ashud_warp_2 false)
                (set `self.IsBossWallEntry` false)))))))))