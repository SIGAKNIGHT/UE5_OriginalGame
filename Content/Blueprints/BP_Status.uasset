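; BP_Status manages a stamina pool with a delayed drain bar and automatic regeneration.
; StaminaConsumption spends stamina only when enough remains, printing a warning otherwise.
; Each Tick, UpdateStamina clamps values, steps TemporalyStamina down toward Stamina after a short delay, and regenerates Stamina gradually after a longer pause.
; Comparing against the previous frame's stamina restarts both delays whenever more is spent.
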(event `self.ReceiveTick`
  (params (DeltaSeconds :type "Float (single-precision)"))
  (`self.UpdateStamina` DeltaSeconds))

(fn `StaminaConsumption`
  (params (Value :type "Float (double-precision)"))
  (returns (Action :type Boolean))
  (locals (bool :type Boolean))
  (bind _output_get (set `local.bool` (> (`self.Stamina`) Value)))
  (if _output_get
    (set `self.Stamina` (- (`self.Stamina`) Value)) ; スタミナを減らす
    (else
      (`KismetSystemLibrary.PrintString` "Need Stamina!" true true (struct :`R` 1.0 :`B` 1.0 :`A` 1.0))))
  (return (`local.bool`)))

(fn `UpdateStamina`
  (params (DeltaSecond :type "Float (double-precision)"))
  (`|ExecutionSequence`
    (:`then_0`
      ;[1 1 1] クランプ
      (set `self.Stamina` (`KismetMathLibrary.FMin` (`self.Stamina`) (`self.MaxStamina`)))
      (set `self.TemporalyStamina` (`KismetMathLibrary.FMin` (`self.TemporalyStamina`) (`self.MaxStamina`))))
    (:`then_1`
      ;[1 1 1] 仮HP計算
      (`self.TemporalyStamina > Stamina`
        (:`true`
          (`self.OldStamina > Stamina`
            (:`true`
              (bind _output_get (set `self.DelayTimer` 0.0)))
            (:`false`
              _))
          (if (>= _output_get 0.1)
            ;;[1 1 1] 仮HPを徐々に減少
            (if (> (`self.DecreaseTimer`) 0.005)
              (`/Engine/EditorBlueprintResources/StandardMacros.DecrementFloat` (`self.TemporalyStamina`)
                (:`  `
                  (set `self.TemporalyStamina` (`KismetMathLibrary.FMax` (`self.Stamina`) (`self.TemporalyStamina`)))
                  (set `self.DecreaseTimer` (- (`self.DecreaseTimer`) (`local.DeltaSecond`))))))
            (set `self.DecreaseTimer` (+ (`self.DecreaseTimer`) (`local.DeltaSecond`))))
          (set `self.DelayTimer` (+ (`self.DelayTimer`) (`local.DeltaSecond`))))
        (:`false`
          (set `self.DelayTimer` 0.0)
          (set `self.DecreaseTimer` 0.0)
          (set `self.TemporalyStamina` (`self.Stamina`)))))
    (:`then_2`
      ;[1 1 1] スタミナ回復
      (`self.Stamina < MaxStamina` ; スタミナがMaxではない
        (:`true`
          (`self.OldStamina > Stamina` ; 追加でダメージを受けていたら
            (:`true`
              (bind _output_get_2 (set `self.HealTimer` 0.0)))
            (:`false`
              _))
          (if (>= _output_get_2 1.5)
            ;;[1 1 1] スタミナを徐々に回復させる
            (if (> (`self.IncreaseTimer`) 0.02)
              (bind _result (`/Engine/EditorBlueprintResources/StandardMacros.IncrementFloat` (`self.Stamina`))
                (:`  `
                  (set `self.Stamina` (`KismetMathLibrary.FMin` _result (`self.MaxStamina`)))
                  (set `self.IncreaseTimer` (- (`self.IncreaseTimer`) 0.02)))))
            (set `self.IncreaseTimer` (+ (`self.IncreaseTimer`) (`local.DeltaSecond`))))
          (set `self.HealTimer` (+ (`self.HealTimer`) (`local.DeltaSecond`))))))
    (:`then_3`
      (set `self.OldStamina` (`self.Stamina`)))))