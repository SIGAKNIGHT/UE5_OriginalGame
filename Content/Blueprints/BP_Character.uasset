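; BP_Character is a character Blueprint that provides small shared helper functions, with empty construction script and event handlers.
; CalcAngle returns the angle in degrees between a front vector and a second vector via the arccosine of their normalized dot product.
; IsFalling wraps the CharacterMovement check, TagCheck tests a target actor for a tag, and StatusPrintString builds a labeled current/max status string.
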(fn `CalcAngle`
  (params (Front :type "Vector Structure") (PtoE :type "Vector Structure"))
  (returns (Degree :type "Float (double-precision)"))
  (return (`KismetMathLibrary.DegAcos` (`KismetMathLibrary.Dot_VectorVector` (`KismetMathLibrary.Normal` Front) (`KismetMathLibrary.Normal` PtoE)))))

(fn `IsFalling`
  (returns (ReturnValue :type Boolean))
  (return (`NavMovementComponent.IsFalling` (`self.CharacterMovement`))))

(fn `StatusPrintString`
  (params (Status :type String) (Current :type "Float (double-precision)") (Max :type "Float (double-precision)"))
  (returns (ReturnValue :type String))
  (return (`KismetStringLibrary.Concat_StrStr` Status (`KismetStringLibrary.Conv_DoubleToString` Current) "/" (`KismetStringLibrary.Conv_DoubleToString` Max))))

(fn `TagCheck`
  (params (`ターゲット` :type "Actor Object Reference") (Tag :type Name))
  (returns (ReturnValue :type Boolean))
  (return (`self.ActorHasTag` `ターゲット` Tag)))

(fn `UserConstructionScript`)