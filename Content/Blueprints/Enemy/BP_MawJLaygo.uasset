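; Enemy character "Taurus Demon", a child of a shared enemy base, with an intro walk and roar plus melee attacks.
; Tick dispatches on an enum state, moving from walk to roar to idle after battle start.
; Punch, swipe, jump attack and backstep events play DoOnce-gated montages, with delayed launches for both leaps.
; Attacks assign damage to child-actor hitboxes on hands and body, owned by the enemy to avoid self-damage.
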(event `self.Active`
  (`parent.Active`))

(event `self.ReceiveBeginPlay`
  (set `self.EnemyName` "Taurus Demon")
  ;[1 1 1] 剣で自分がダメージを受けないようにする
  (`self.SetOwner` (`ChildActorComponent.ChildActor` (`self.L_Weapon`)) self)
  (`self.SetOwner` (`ChildActorComponent.ChildActor` (`self.R_Weapon`)) self)
  (`self.SetOwner` (`ChildActorComponent.ChildActor` (`self.Body`)) self)
  (`parent.ReceiveBeginPlay`))

(event `self.ReceiveTick`
  (params (DeltaSeconds :type "Float (single-precision)"))
  ;[1 1 1] Tick
  (`parent.ReceiveTick` DeltaSeconds)
  (switch `/Game/Blueprints/Enemy/EnemyEnum` (`self.EnemyEnum`)
    (:`NewEnumerator1`
      (`self.WalkForward`))
    (:`NewEnumerator2`
      (`self.Roar`))))

(event `self.BattleStart`
  (`/Engine/EditorBlueprintResources/StandardMacros.DoOnce` false
    (:`Completed`
      (set `self.EnemyEnum` "NewEnumerator1"))))

(event `self.Death`
  (params (MontageToPlay :type "AnimMontage Object Reference"))
  (`parent.Death` "/Game/AnimMontage/MawJLaygo/StandingReactDeathForward_UE_Montage.StandingReactDeathForward_UE_Montage"))

(event `WalkForward`
  (`self.Move` 0.0 1.0)
  (`/Engine/EditorBlueprintResources/StandardMacros.DoOnce` false
    (:`Completed`
      (`KismetSystemLibrary.Delay` 0.75)
      (set `self.EnemyEnum` "NewEnumerator2"))))

(event `Roar`
  (if (not (`self.IsFalling`))
    (`KismetSystemLibrary.Delay` 0.75)
    (`/Engine/EditorBlueprintResources/StandardMacros.DoOnce` false :!label _label
      (:`Completed`
        (`KismetSystemLibrary.PrintString` "DoOnce")
        (`|PlayMontage` (`self.Mesh`) "/Game/AnimMontage/MawJLaygo/mutantroaring_UE_Montage.mutantroaring_UE_Montage" 1.5
          (:`OnCompleted`
            _)
          (:`OnInterrupted`
            _))
        (set `self.IsFirstAction` true)
        (set `self.EnemyEnum` "NewEnumerator3")
        (`KismetSystemLibrary.Delay` 1.0)
        (goto _label :!via `Reset`)))))

(event `self.AttackR1`
  ;[1 1 1] R1
  (`/Engine/EditorBlueprintResources/StandardMacros.DoOnce` false :!label _label_2
    (:`Completed`
      (`self.SetPunchDamage` (`self.R_Weapon`) 150.0)
      (`|PlayMontage` (`self.Mesh`) "/Game/AnimMontage/MawJLaygo/mutantpunch_UE_Montage.mutantpunch_UE_Montage"
        (:`OnCompleted`
          (goto _label_2 :!via `Reset`))
        (:`OnInterrupted`
          (goto _label_2 :!via `Reset`))))))

(event `self.AttackR2`
  ;[1 1 1] R2
  (`/Engine/EditorBlueprintResources/StandardMacros.DoOnce` false :!label _label_3
    (:`Completed`
      (`self.SetDamage` (`self.L_Weapon`) 250.0)
      (`|PlayMontage` (`self.Mesh`) "/Game/AnimMontage/MawJLaygo/mutantswiping_UE_Montage.mutantswiping_UE_Montage"
        (:`OnCompleted`
          (goto _label_3 :!via `Reset`))
        (:`OnInterrupted`
          (goto _label_3 :!via `Reset`))))))

(event `self.AttackJump`
  (`/Engine/EditorBlueprintResources/StandardMacros.DoOnce` false :!label _label_4
    (:`Completed`
      (`self.SetDamage` (`self.Body`) 300.0)
      (`self.SetDamage` (`self.L_Weapon`) 0.0)
      (`self.SetDamage` (`self.R_Weapon`) 0.0)
      (`|PlayMontage` (`self.Mesh`) "/Game/AnimMontage/MawJLaygo/mutantjumpattack_UE_Montage.mutantjumpattack_UE_Montage"
        (:`then`
          (`KismetSystemLibrary.Delay` 0.75)
          (`self.FC_LaunchCharacter` 500.0 500.0))
        (:`OnCompleted`
          (goto _label_4 :!via `Reset`))
        (:`OnInterrupted`
          (goto _label_4 :!via `Reset`))))))

(event `self.BackStep`
  (`/Engine/EditorBlueprintResources/StandardMacros.DoOnce` false :!label _label_5
    (:`Completed`
      (`|PlayMontage` (`self.Mesh`) "/Game/AnimMontage/MawJLaygo/mutantjumping_UE_Montage.mutantjumping_UE_Montage" 1.5
        (:`then`
          (`KismetSystemLibrary.Delay` 0.75)
          (`self.FC_LaunchCharacter` -500.0 500.0))
        (:`OnCompleted`
          (goto _label_5 :!via `Reset`))
        (:`OnInterrupted`
          (goto _label_5 :!via `Reset`))))))

(fn `FC_LaunchCharacter`
  (params (XY_Value :type "Float (double-precision)") (Z_Value :type "Float (double-precision)"))
  (`parent.FC_LaunchCharacter` XY_Value Z_Value))

(fn `IsTargetable`
  (returns (ReturnValue :type Boolean))
  (return (`self.IsActive`)))

(fn `SetDamage`
  (params (Actor :type "ChildActorComponent Object Reference") (Damage :type "Float (double-precision)"))
  (bind _childactor (`ChildActorComponent.ChildActor` Actor))
  (bind _asbp_punch (cast `/Game/Blueprints/Weapon/BP_Punch` _childactor)
    (:`then`
      (set `/Game/Blueprints/Weapon/BP_BaseWeapon.Damage` Damage _asbp_punch))
    (:`CastFailed`
      (bind _asbp_body_press (cast `/Game/Blueprints/Weapon/BP_BodyPress` _childactor)
        (:`then`
          (set `/Game/Blueprints/Weapon/BP_BaseWeapon.Damage` Damage _asbp_body_press))
        (:`CastFailed`
          (`KismetSystemLibrary.PrintString` "Cast Failed" true true (struct :`R` 1.0 :`B` 1.0 :`A` 1.0)))))))

(fn `SetJumpDamage`
  (params (Actor :type "ChildActorComponent Object Reference") (Damage :type "Float (double-precision)"))
  (bind _asbp_body_press (cast `/Game/Blueprints/Weapon/BP_BodyPress` (`ActorComponent.GetOwner` Actor)))
  (set `/Game/Blueprints/Weapon/BP_BaseWeapon.Damage` Damage _asbp_body_press))

(fn `SetPunchDamage`
  (params (Actor :type "ChildActorComponent Object Reference") (Damage :type "Float (double-precision)"))
  (bind _asbp_punch (cast `/Game/Blueprints/Weapon/BP_Punch` (`ActorComponent.GetOwner` Actor)))
  (set `/Game/Blueprints/Weapon/BP_BaseWeapon.Damage` Damage _asbp_punch))

(fn `UserConstructionScript`
  (`parent.UserConstructionScript`))