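; BP_FP manages the player's FP (stamina-like) pool, filling it on BeginPlay and keeping a trailing TemporalyFP value that lags behind spending.
; Each Tick, UpdateFP caps both values at MaxFP and holds TemporalyFP briefly after a drop before draining it toward FP at a frame-rate-independent rate.
; Further drops during the lag, detected via OldFP, restart the delay.
; Despite its name, HPConsumption spends FP, returning whether enough was available.
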(event `self.ReceiveBeginPlay`
  (set `self.FP` (`self.MaxFP`)))

(event `self.ReceiveTick`
  (params (DeltaSeconds :type "Float (single-precision)"))
  (`self.UpdateFP` DeltaSeconds))

(fn `HPConsumption`
  (params (Value :type "Float (double-precision)"))
  (returns (Action :type Boolean))
  (locals (bool :type Boolean))
  (bind _output_get (set `local.bool` (> (`self.FP`) Value)))
  (if _output_get
    (set `self.FP` (- (`self.FP`) Value)) ; スタミナを減らす
    (else
      (`KismetSystemLibrary.PrintString` "Need Stamina!" true true (struct :`R` 1.0 :`B` 1.0 :`A` 1.0))))
  (return (`local.bool`)))

(fn `UpdateFP`
  (params (ElapsedTime :type "Float (double-precision)"))
  (`|ExecutionSequence`
    (:`then_0`
      ;[1 1 1] クランプ
      (set `self.FP` (`KismetMathLibrary.FMin` (`self.FP`) (`self.MaxFP`)))
      (set `self.TemporalyFP` (`KismetMathLibrary.FMin` (`self.TemporalyFP`) (`self.MaxFP`))))
    (:`then_2`
      ;[1 1 1] 仮FP計算
      (`self.TemporalyFP > FP` ; FP消費後なら
        (:`true`
          (`self.OldFP > FP` ; 再度FPを消費していたら
            (:`true`
              (set `self.TemporalyFP` (`self.OldFP`))
              (bind _output_get (set `self.DelayTimer` 0.0)))
            (:`false`
              _))
          (if (>= _output_get 1.0)
            (set `self.TemporalyFP` (`KismetMathLibrary.FMax` (`self.FP`) (- (`self.TemporalyFP`) (`self.FloatPerFrame` 200.0 (`local.ElapsedTime`))))))
          (set `self.DelayTimer` (+ (`self.DelayTimer`) (`local.ElapsedTime`))))
        (:`false`
          (set `self.DelayTimer` 0.0)
          (set `self.TemporalyFP` (`self.FP`)))))
    (:`then_4`
      (set `self.OldFP` (`self.FP`)))))