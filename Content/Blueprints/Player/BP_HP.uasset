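; Player HP Blueprint that tracks health, an invincibility countdown and a delayed "temporary HP" value that trails damage.
; Each tick clamps HP to its maximum, counts down invincibility, then drains temporary HP toward HP at a fixed rate after a delay.
; Further damage snaps temporary HP to the previous HP and restarts the delay.
; HPConsumption spends HP only if enough remains; an enemy fast-decrease variant is left unconnected.
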(event `self.ReceiveBeginPlay`
  (set `self.HP` (`self.MaxHP`)))

(event `self.ReceiveTick`
  (params (DeltaSeconds :type "Float (single-precision)"))
  (`self.UpdateHP` DeltaSeconds))

(fn `HPConsumption`
  (params (Value :type "Float (double-precision)"))
  (returns (Action :type Boolean))
  (locals (bool :type Boolean))
  (bind _output_get (set `local.bool` (> (`self.HP`) Value)))
  (if _output_get
    (set `self.HP` (- (`self.HP`) Value)) ; スタミナを減らす
    (else
      (`KismetSystemLibrary.PrintString` "Need Stamina!" true true (struct :`R` 1.0 :`B` 1.0 :`A` 1.0))))
  (return (`local.bool`)))

(fn `Update_Invincible_Timer`
  (params (elapsedTime :type "Float (double-precision)"))
  (if (> (`self.Invincible_Timer`) 0.0)
    (set `self.Invincible_Timer` (`KismetMathLibrary.FMax` (- (`self.Invincible_Timer`) (`local.elapsedTime`))))
    (return)
    (else
      (return))))

(fn `UpdateHP`
  (params (ElapsedTime :type "Float (double-precision)"))
  (`|ExecutionSequence`
    (:`then_0`
      ;[1 1 1] クランプ
      (set `self.HP` (`KismetMathLibrary.FMin` (`self.HP`) (`self.MaxHP`)))
      (set `self.TemporalyHP` (`KismetMathLibrary.FMin` (`self.TemporalyHP`) (`self.MaxHP`))))
    (:`then_1`
      (`self.Update_Invincible_Timer` (`local.ElapsedTime`)))
    (:`then_2`
      ;[1 1 1] 仮HP計算
      (`self.TemporalyHP > HP` ; ダメージを受けた後なら
        (:`true`
          (`self.OldHP > HP` ; 再度ダメージを受けていたら
            (:`true`
              (set `self.TemporalyHP` (`self.OldHP`))
              (bind _output_get (set `self.DelayTimer` 0.0)))
            (:`false`
              _))
          (if (>= _output_get 4.0)
            (set `self.TemporalyHP` (`KismetMathLibrary.FMax` (`self.HP`) (- (`self.TemporalyHP`) (`self.FloatPerFrame` 200.0 (`local.ElapsedTime`))))))
          (set `self.DelayTimer` (+ (`self.DelayTimer`) (`local.ElapsedTime`))))
        (:`false`
          (set `self.DelayTimer` 0.0)
          (set `self.TemporalyHP` (`self.HP`)))))
    (:`then_4`
      (set `self.OldHP` (`self.HP`)))))