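; BP_MawJLaygo is an enemy Blueprint that names itself "Taurus Demon" and dies automatically shortly after play begins.
; BeginPlay sets EnemyName before calling the parent's BeginPlay, then waits on a fixed delay and fires Death.
; Death and the construction script only forward to the parent class, which supplies the actual behavior.
; The Tick and overlap events are disabled placeholders.
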(event `self.ReceiveBeginPlay`
  (set `self.EnemyName` "Taurus Demon")
  (`parent.ReceiveBeginPlay`)
  (`KismetSystemLibrary.Delay` 7.0)
  (`self.Death` null))

(event `self.Death`
  (params (MontageToPlay :type "AnimMontage Object Reference"))
  (`parent.Death` null))

(fn `UserConstructionScript`
  (`parent.UserConstructionScript`))