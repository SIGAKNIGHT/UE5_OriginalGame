(event `self.ReceiveBeginPlay`
  (`parent.ReceiveBeginPlay`)
  (`|ExecutionSequence`
    (:`then_1`
      ;[1 1 1] HPゲージ作成
      (bind _returnvalue (`|CreateWidget` "/Game/MaedaDaiki/Blueprints/BossHP_WBP.BossHP_WBP_C"))
      (bind _output_get (set `self.BossHP_Widget` _returnvalue))
      (`Widget.SetVisibility` _output_get "Hidden")
      (`UserWidget.AddToViewport` _output_get 0))
    (:`then_2`
      ;[1 1 1] 名前設定
      (`/Game/MaedaDaiki/Blueprints/BossHP_WBP.DispSetEnemyName_Event` (`self.BossHP_Widget`) (`self.EnemyName`)))))

(event `self.ReceiveAnyDamage`
  (params (Damage :type "Float (single-precision)") (DamageType :type "DamageType Object Reference") (InstigatedBy :type "Controller Object Reference") (DamageCauser :type "Actor Object Reference"))
  (bind _bp_hp (`self.BP_HP`))
  ;[1 1 1] 被ダメージ
  (bind _output_get (set `/Game/Blueprints/Player/BP_HP.HP` (- (`/Game/Blueprints/Player/BP_HP.HP` _bp_hp) Damage) _bp_hp))
  (if (not (> _output_get 0.0))
    (`self.Death`)))

(event `Death`
  ;[1 1 1] 死亡時
  (bind _ashud_warp (cast `/Game/MaedaDaiki/Blueprints/HUD_Warp` (`PlayerController.GetHUD` (`GameplayStatics.GetPlayerController` 0))))
  (`/Game/MaedaDaiki/Blueprints/HUD_Warp.DispYouHunted_Event` _ashud_warp))

(event `self.ReceiveTick`
  (params (DeltaSeconds :type "Float (single-precision)"))
  (`parent.ReceiveTick` DeltaSeconds)
  (`|ExecutionSequence`
    (:`then_0`
      (`self.HUD_Clamp`))
    (:`then_1`
      ;[1 1 1] プレイヤー霧抜け判定
      (`/Engine/EditorBlueprintResources/StandardMacros.DoOnce` false :!label _label
        (:`Completed`
          (bind _asbp_player (cast `/Game/Blueprints/Player/BP_Player` (`GameplayStatics.GetPlayerCharacter` 0)))
          (if (`/Game/MaedaDaiki/Blueprints/BossWallEntry.IsInBossStage` (`/Game/Blueprints/Player/BP_Player.BossWallEntry` _asbp_player))
            (set `self.Active` true)
            (`Widget.SetVisibility` (`self.BossHP_Widget`) "Visible")
            (else
              (goto _label :!via `Reset`))))))))

(fn `HUD_Clamp`
  (bind _bp_hp (`self.BP_HP`))
  (bind _bp_hp_2 (`self.BP_HP`))
  (bind _totaldamage (`/Game/Blueprints/Player/BP_HP.TotalDamage` (`self.BP_HP`)))
  ;[1 1 1] HP系を0~1にクランプ
  (`|ExecutionSequence`
    (:`then_0`
      (set `/Game/MaedaDaiki/Blueprints/BossHP_WBP.WBP_HP` (/ (`/Game/Blueprints/Player/BP_HP.HP` _bp_hp) (`/Game/Blueprints/Player/BP_HP.MaxHP` _bp_hp)) (`self.BossHP_Widget`)))
    (:`then_1`
      (set `/Game/MaedaDaiki/Blueprints/BossHP_WBP.WBP_LastHP` (/ (`/Game/Blueprints/Player/BP_HP.LastHP` _bp_hp_2) (`/Game/Blueprints/Player/BP_HP.MaxHP` _bp_hp_2)) (`self.BossHP_Widget`)))
    (:`then_2`
      (set `/Game/MaedaDaiki/Blueprints/BossHP_WBP.WBP_BossDamage` (`KismetMathLibrary.FTrunc` _totaldamage) (`self.BossHP_Widget`))
      (`KismetSystemLibrary.PrintString` (`KismetStringLibrary.Conv_DoubleToString` _totaldamage) true false (struct :`R` 0.6 :`A` 1.0) 0.0))))

(fn `UserConstructionScript`
  (`parent.UserConstructionScript`))